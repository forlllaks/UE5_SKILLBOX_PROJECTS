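; BP_TraffictLight is a traffic light actor whose light color follows its current state.
; On BeginPlay it creates a dynamic material instance of M_TrafficColorInstance on the Light component's first material slot.
; The ChangeColor event stores the new state, looks it up in the LightColorSettings color map, and, when found, sets the material's Color parameter to the mapped color.
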(event `self.ReceiveBeginPlay`
  (`|ExecutionSequence`
    (:`then_0`
      (bind _returnvalue (`PrimitiveComponent.CreateDynamicMaterialInstance` (`self.Light`) 0 "/Game/Blueprints/Materials/M_TrafficColorInstance.M_TrafficColorInstance" "None"))
      (set `self.Material` _returnvalue))))

(event `ChangeColor`
  (params (NewState :type "/Game/Blueprints/E_LightColor Enum" :default "NewEnumerator0"))
  (bind _lightcolorsettings_colormap (break `/Game/Blueprints/S_LIghtColorSetting` (`self.LightColorSettings`)))
  (bind _output_get (set `self.State` NewState))
  (bind (_value _returnvalue) (`BlueprintMapLibrary.Map_Find` _lightcolorsettings_colormap _output_get))
  (if _returnvalue
    (`MaterialInstanceDynamic.SetVectorParameterValue` (`self.Material`) "Color" (break `/Game/Blueprints/S_LightColor` _value))))

(fn `UserConstructionScript`)