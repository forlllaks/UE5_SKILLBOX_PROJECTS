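; Manager that cycles every BP_TraffictLight actor in the level through a shared traffic light sequence.
; Recolor steps CurrentColor back and forth between Red, Yellow and Green, reversing at either end.
; It pushes the color to all lights, swapping Red and Green for those flagged InTwoSide.
; Tick drives a DoOnce-gated Delay, timed per color from ColorSettings, that calls Recolor and then resets the gate.
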(event `self.ReceiveBeginPlay`
  (`self.Recolor`))

(event `self.ReceiveTick`
  (params (DeltaSeconds :type "Float (single-precision)"))
  (`self.TickLive`))

(event `Recolor`
  (bind _currentcolor (`self.CurrentColor`))
  (bind _currentcolor_2 (`self.CurrentColor`))
  (`|ExecutionSequence`
    (:`then_0`
      ;[0.5999 0.5473 1] Смотрим если это конец листа то меняем направление.
      (switch `/Game/Blueprints/E_LightColor` (`self.CurrentColor`)
        (:`NewEnumerator0`
          (set `self.ReverseColorSelection` false))
        (:`NewEnumerator2`
          (set `self.ReverseColorSelection` true))))
    (:`then_1`
      ;[1 0.9799 0.4943] Меняем цвет на следующий
      (if (`self.ReverseColorSelection`)
        (set `self.CurrentColor` (cast `/Game/Blueprints/E_LightColor` (- _currentcolor 1)))
        (else
          (set `self.CurrentColor` (cast `/Game/Blueprints/E_LightColor` (+ _currentcolor 1)))))
      ;[0.2242 1 0] Меняем у всех светофоров  цвета
      (bind _outactors (`GameplayStatics.GetAllActorsOfClass` "/Game/Blueprints/BP_TraffictLight.BP_TraffictLight_C"))
      (for _array_element _outactors
        (if (`/Game/Blueprints/BP_TraffictLight.InTwoSide?` _array_element)
          (switch `/Game/Blueprints/E_LightColor` _currentcolor_2
            (:`NewEnumerator0`
              (`/Game/Blueprints/BP_TraffictLight.ChangeColor` _array_element "NewEnumerator2"))
            (:`NewEnumerator1`
              (`/Game/Blueprints/BP_TraffictLight.ChangeColor` _array_element "NewEnumerator1"))
            (:`NewEnumerator2`
              (`/Game/Blueprints/BP_TraffictLight.ChangeColor` _array_element "NewEnumerator0")))
          (else
            (`/Game/Blueprints/BP_TraffictLight.ChangeColor` _array_element _currentcolor_2)))))))

(event `TickLive`
  ;[0.6756 1 0.1718] Меняем цвет через заданное время
  (`/Engine/EditorBlueprintResources/StandardMacros.DoOnce` false :!label _label
    (:`Completed`
      (`KismetSystemLibrary.Delay` (`.Timer_7_438B950D4897E330A30927AAD7151930` (break `/Game/Blueprints/S_LightColor` (`BlueprintMapLibrary.Map_Find` (`.ColorMap_10_AD10A8064177A299623046ADAA65AF4C` (break `/Game/Blueprints/S_LIghtColorSetting` (`self.ColorSettings`))) (`self.CurrentColor`)))))
      (`self.Recolor`)
      (goto _label :!via `Reset`))))

(fn `UserConstructionScript`)